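; PawnBP is the camera pawn of the SimpleRoleChange project, providing an orbit and zoom view alongside a character creation UI.
; Mouse X and Y axes feed controller yaw and pitch to rotate the view.
; The mouse wheel steps the SpringArm length within clamped near and far limits.
; BeginPlay creates the CreatePlayer_UI widget and adds it to the viewport.
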(event EventBeginPlay
  ;[0 0 0] 显示界面
  (bind _returnvalue (UserInterface|CreateWidget "/Game/SimpleRoleChange/UI/CreatePlayer_UI.CreatePlayer_UI_C"))
  (UserInterface|Viewport|AddtoViewport _returnvalue 0))

(event Input|MouseEvents|MouseX
  (params (AxisValue :type Float%20%28single-precision%29))
  ;[0 0 0] 摄像机控制旋转
  (Pawn|Input|AddControllerYawInput AxisValue))

(event Input|MouseEvents|MouseY
  (params (AxisValue :type Float%20%28single-precision%29))
  ;[0 0 0] 摄像机控制旋转
  (Pawn|Input|AddControllerPitchInput AxisValue))

(event Input|MouseEvents|MouseWheelUp
  (params (Key :type Key%20Structure :default "None"))
  ;[0 0 0] 鼠标滚轮缩放视角
  (:Pressed
    (Variables|/Script/Engine.SpringArmComponent|SetTargetArmLength (Variables|Default|GetSpringArm) (Math|Float|Clamp(Float) (- (Variables|/Script/Engine.SpringArmComponent|GetTargetArmLength (Variables|Default|GetSpringArm)) 15.0) 1.5e+02 3e+02))))

(event Input|MouseEvents|MouseWheelDown
  (params (Key :type Key%20Structure :default "None"))
  ;[0 0 0] 鼠标滚轮缩放视角
  (:Pressed
    (Variables|/Script/Engine.SpringArmComponent|SetTargetArmLength (Variables|Default|GetSpringArm) (Math|Float|Clamp(Float) (+ (Variables|/Script/Engine.SpringArmComponent|GetTargetArmLength (Variables|Default|GetSpringArm)) 15.0) 1.5e+02 3e+02))))

(fn ConstructionScript)